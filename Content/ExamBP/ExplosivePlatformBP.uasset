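; An explosive platform actor that counts down and blows up after something overlaps it.
; Each overlap calls Countdown, which decrements Time and re-calls itself after a one-second Delay, so repeated overlaps also decrement the timer.
; When Time runs out it plays an explosion sound, destroys its mesh, spawns an explosion effect Blueprint at the root's location and destroys itself.
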(event Custom|Countdown
  (bind _defaultsceneroot (Variables|Default|GetDefaultSceneRoot))
  (bind _returnvalue (Transformation|GetWorldLocation _defaultsceneroot))
  (Math|Float|DecrementFloat (Variables|Default|GetTime)
    (:%20%20
      (if (<= (Variables|Default|GetTime) 0.0)
        (Audio|PlaySoundatLocation "/Game/StarterContent/Audio/Explosion01.Explosion01" _returnvalue)
        (Components|DestroyComponent (Variables|Default|GetStaticMesh))
        (Game|SpawnActorfromClass "/Game/StarterContent/Blueprints/Blueprint_Effect_Explosion.Blueprint_Effect_Explosion_C" (Math|Transform|MakeTransform _returnvalue "0, 0, 0" "1,1,1") "Undefined" 0 0)
        (Actor|DestroyActor (Components|GetOwner (Variables|Default|GetDefaultSceneRoot)))
        (else
          (Utilities|FlowControl|Delay 1.0)
          (CallFunction|Countdown))))))

(event Collision|EventActorBeginOverlap
  (params (OtherActor :type Actor%20Object%20Reference))
  (CallFunction|Countdown))

(fn ConstructionScript)