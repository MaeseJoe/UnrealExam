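; InsecurePlatformBP is a platform that fades away and destroys itself once the third-person character touches it.
; The construction script creates a dynamic material instance from InsecureMatInstance on the static mesh.
; An overlap with ThirdPersonCharacter plays a timeline that drives the material's Opacity parameter, destroying the actor when opacity reaches zero.
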(event Custom|DisappearEvt
  (bind _opacityreduction (Timeline|Timeline_0 Play)
    (:Update
      (Rendering|Material|SetScalarParameterValueonMaterials (Variables|Default|GetStaticMesh) "Opacity" _opacityreduction)
      (if (<= _opacityreduction 0.0)
        (Actor|DestroyActor (Components|GetOwner (Variables|Default|GetDefaultSceneRoot)))))))

(event Collision|EventActorBeginOverlap
  (params (OtherActor :type Actor%20Object%20Reference))
  (Utilities|Casting|CastToThirdPersonCharacter OtherActor)
  (CallFunction|DisappearEvt))

(fn ConstructionScript
  (Rendering|Material|CreateDynamicMaterialInstance (Variables|Default|GetStaticMesh) 0 "/Game/ExamMat/InsecureMatInstance.InsecureMatInstance" :!class /Script/Engine.PrimitiveComponent))